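; BP_EchoPulse is a one-shot echolocation pulse that briefly reveals tagged objects as it spreads.
; On BeginPlay, a timeline grows a flat ring mesh and a collision sphere together, then destroys the actor.
; Overlapped actors tagged EchoReveal get their static mesh material swapped to white, then to black after a short Delay.
; Debug strings print along the way.
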(event `self.ReceiveBeginPlay`
  (bind (_direction _alpha) (`Timeline|TL_EchoExpand` :!via `PlayFromStart`)
    (:`Update`
      (bind _returnvalue (`KismetMathLibrary.Lerp` 0.1 20.0 _alpha))
      (`SceneComponent.SetWorldScale3D` (`self.EchoRing`) (`KismetMathLibrary.MakeVector` _returnvalue _returnvalue 0.02))
      (`SphereComponent.SetSphereRadius` (`self.EchoCollision`) (`KismetMathLibrary.Lerp` 50.0 1200.0 _alpha) true))
    (:`Finished`
      (`self.K2_DestroyActor`))))

(event `self.EchoCollision.OnComponentBeginOverlap`
  (params (OverlappedComponent :type "PrimitiveComponent Object Reference") (OtherActor :type "Actor Object Reference") (OtherComp :type "PrimitiveComponent Object Reference") (OtherBodyIndex :type Integer) (bFromSweep :type Boolean) (SweepResult :type "HitResult Structure (by ref)"))
  (bind _returnvalue (`self.GetComponentByClass` OtherActor "/Script/Engine.StaticMeshComponent"))
  (`KismetSystemLibrary.PrintString` "Overlap")
  (if (`self.ActorHasTag` OtherActor "EchoReveal")
    (`KismetSystemLibrary.PrintString` (`KismetSystemLibrary.GetDisplayName` OtherActor))
    (`KismetSystemLibrary.PrintString` "Reveal wall")
    (`PrimitiveComponent.SetMaterial` _returnvalue 0 "/Game/Materials/M_Echo_Reveal_White.M_Echo_Reveal_White")
    (`KismetSystemLibrary.Delay` 0.6)
    (`PrimitiveComponent.SetMaterial` _returnvalue 0 "/Game/Materials/M_Env_Black.M_Env_Black")
    (`KismetSystemLibrary.PrintString` "Set wall black")))

(fn `UserConstructionScript`)